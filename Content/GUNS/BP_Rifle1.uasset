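; BP_Rifle1 is a rifle gun actor that can be picked up when another actor overlaps it.
; The construction script sets its spread, fire rate and magazine size.
; A boolean condition turns off its rotating movement at start and blocks the pickup call, which runs after a short delay on overlap.
; Each tick it copies an arrow component's relative transform as the bullet spawn transform.
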(event `self.ReceiveBeginPlay`
  (`KismetSystemLibrary.DelayUntilNextTick`)
  (if (`self.Condition`)
    (`ActorComponent.SetActive` (`self.RotatingMovement`) false false)))

(event `self.ReceiveActorBeginOverlap`
  (params (OtherActor :type "Actor Object Reference"))
  (`KismetSystemLibrary.Delay` 0.1)
  (if (not (`self.Condition`))
    (`self.PickedUp` self OtherActor)))

(event `self.ReceiveTick`
  (params (DeltaSeconds :type "Float (single-precision)"))
  (set `self.BulletSpawnTransform` (`SceneComponent.GetRelativeTransform` (`self.Arrow`))))

(fn `UserConstructionScript`
  (set `self.Spread` 5)
  (set `self.FireRate` 17.0)
  (set `self.MagSize` 30))