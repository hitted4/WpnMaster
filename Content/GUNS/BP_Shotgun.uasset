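; BP_Shotgun is a shotgun gun actor that sets its weapon stats, such as spread, fire rate and magazine size, in the construction script.
; Overlapping it calls PickedUp after a short delay when a condition is false.
; On BeginPlay it waits a tick, then conditionally disables its RotatingMovement.
; Tick uses a short Delay to refresh the bullet spawn transform from the Arrow's relative transform.
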(event `self.ReceiveBeginPlay`
  (`KismetSystemLibrary.DelayUntilNextTick`)
  (if (`self.Condition`)
    (`ActorComponent.SetActive` (`self.RotatingMovement`) false false)))

(event `self.ReceiveActorBeginOverlap`
  (params (OtherActor :type "Actor Object Reference"))
  (`KismetSystemLibrary.Delay` 0.1)
  (if (not (`self.Condition`))
    (`self.PickedUp` self OtherActor)))

(event `self.ReceiveTick`
  (params (DeltaSeconds :type "Float (single-precision)"))
  (`KismetSystemLibrary.Delay` 0.016666)
  (set `self.BulletSpawnTransform` (`SceneComponent.GetRelativeTransform` (`self.Arrow`))))

(fn `UserConstructionScript`
  (set `self.Spread` 12)
  (set `self.FireRate` 2.0)
  (set `self.MagSize` 15)
  (set `self.Type` "Shotgun")
  (set `self.Range` 10.0))