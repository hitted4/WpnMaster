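; Rifle bullet projectile that detects hits by tracing along its travelled path instead of relying on overlaps.
; A short delay on Tick paces Visibility line traces from the last stored position to the Box's current location, ignoring the player pawn and drawing debug lines.
; A hit prints the actor's name and destroys the bullet, with no damage applied; a miss stores the position and re-arms the DoOnce gate.
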(event `self.ReceiveTick`
  (params (DeltaSeconds :type "Float (single-precision)"))
  (bind _returnvalue (`SceneComponent.K2_GetComponentLocation` (`self.Box`)))
  (`KismetSystemLibrary.Delay` 0.01666)
  (`/Engine/EditorBlueprintResources/StandardMacros.DoOnce` false :!label _label
    (:`Completed`
      (bind (_outhit _returnvalue_2) (`KismetSystemLibrary.LineTraceSingle` (`self.LastPos`) _returnvalue "TraceTypeQuery1" false (`|MakeArray` (`GameplayStatics.GetPlayerPawn` 0) :!type "Actor Object Reference") "ForOneFrame" true (struct :`R` 1.0 :`A` 1.0) (struct :`G` 1.0 :`A` 1.0) 2.0))
      (if _returnvalue_2
        (`KismetSystemLibrary.PrintString` (`KismetSystemLibrary.GetDisplayName` (`.HitActor` (`GameplayStatics.BreakHitResult` _outhit))) true false)
        (`self.K2_DestroyActor`)
        (else
          (set `self.LastPos` _returnvalue)
          (goto _label :!via `Reset`))))))

(event `self.ReceiveBeginPlay`
  (set `self.LastPos` (`SceneComponent.K2_GetComponentLocation` (`self.Box`))))

(fn `UserConstructionScript`)